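; Enemy AI controller that starts the BT_AI behavior tree with the BB_AI blackboard and feeds it perception results.
; Successfully sensing the first player's pawn sets IsPlayerVisible and TargetActor.
; Successfully sensing any other actor clears IsPlayerVisible and stores the player's current position as LastKnownLocation.
; Failed stimuli, such as losing sight of the player, leave the blackboard unchanged.
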(event OnTargetPerceptionUpdated(AIPerception)
  (params (Actor :type Actor%20Object%20Reference) (Stimulus :type AI%20Stimulus%20Structure))
  (bind _returnvalue (Game|Player|GetPlayerPawn 0))
  (bind _returnvalue_2 (AI|GetBlackboard 0))
  (bind _returnvalue_3 (Utilities|Name|MakeLiteralName "IsPlayerVisible"))
  (if (.bSuccessfullySensed (Utilities|Struct|BreakAIStimulus Stimulus))
    (if (== Actor _returnvalue)
      (AI|Components|Blackboard|SetValueasBool _returnvalue_2 _returnvalue_3 true)
      (AI|Components|Blackboard|SetValueasObject _returnvalue_2 (Utilities|Name|MakeLiteralName "TargetActor") Actor)
      (else
        (AI|Components|Blackboard|SetValueasBool _returnvalue_2 _returnvalue_3 false)
        (AI|Components|Blackboard|SetValueasVector _returnvalue_2 (Utilities|Name|MakeLiteralName "LastKnownLocation") (Transformation|GetActorLocation _returnvalue))))))

(event EventBeginPlay
  (Class|AIController|UseBlackboard "/Game/EnemyAI/BB_AI.BB_AI")
  (AI|RunBehaviorTree "/Game/EnemyAI/BT_AI.BT_AI"))

(fn ConstructionScript)