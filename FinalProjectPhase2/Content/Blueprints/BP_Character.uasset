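; BP_Character is the player character Blueprint, handling input setup, HUD creation and a pause menu toggle.
; BeginPlay adds the default Enhanced Input mapping context, shows health and speed widgets, and copies Health and Stamina from BP_GameInstance.
; The pause input adds or removes a LevelWidget menu, switching input mode and mouse cursor through an IsPaused flag, without actually pausing the game.
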(event Input|EnhancedActionEvents|EnhancedInputActionIA_Pause
  (params (ActionValue :type Boolean) (ElapsedSeconds :type Float%20%28double-precision%29) (TriggeredSeconds :type Float%20%28double-precision%29) (InputAction :type Input%20Action%20Object%20Reference :default "/Game/Input/Actions/IA_Pause.IA_Pause"))
  (bind _returnvalue (Game|GetPlayerController 0))
  (:Started
    (if (Variables|Default|GetbIsPaused)
      (Input|SetInputModeGameOnly _returnvalue false)
      (Widget|RemovefromParent (Variables|Default|GetMenuWidget))
      (Variables|/Script/Engine.PlayerController|SetbShowMouseCursor _returnvalue false)
      (Variables|Default|SetbIsPaused false)
      (else
        (Input|SetInputModeGameandUI _returnvalue 0 "DoNotLock" true false)
        (bind _returnvalue_2 (UserInterface|CreateWidget "/Game/UI/LevelWidget.LevelWidget_C"))
        (bind _output_get (Variables|Default|SetMenuWidget _returnvalue_2))
        (UserInterface|Viewport|AddtoViewport _output_get 0)
        (Variables|/Script/Engine.PlayerController|SetbShowMouseCursor _returnvalue true)
        (Variables|Default|SetbIsPaused true)))))

(event EventBeginPlay
  (Utilities|FlowControl|Sequence
    (:then_0
      (bind _returnvalue (Class|InputDeviceLibrary|GetPlayerControllerfromInputDevice))
      (Input|AddMappingContext (PlayerController|LocalPlayerSubsystems|GetEnhancedInputLocalPlayerSubsystem _returnvalue) "/Game/Input/IMC_Default.IMC_Default" 0 "(bIgnoreAllPressedKeysUntilRelease=True,bForceImmediately=False,bNotifyUserSettings=False)")
      (bind _returnvalue_2 (UserInterface|CreateWidget "/Game/UI/HealthWidget.HealthWidget_C"))
      (bind _returnvalue_3 (UserInterface|CreateWidget "/Game/UI/SpeedWidget.SpeedWidget_C"))
      (UserInterface|Viewport|AddtoViewport _returnvalue_3 0)
      (bind _asbp_game_instance (Utilities|Casting|CastToBP_GameInstance (Game|GetGameInstance)))
      (Variables|Default|SetHealth (Variables|/Game/Blueprints/BP_GameInstance.BP_GameInstance_C|GetGI_Health _asbp_game_instance))
      (Variables|Default|SetStamina (Variables|/Game/Blueprints/BP_GameInstance.BP_GameInstance_C|GetGI_Stamina _asbp_game_instance)))))

(fn ConstructionScript)