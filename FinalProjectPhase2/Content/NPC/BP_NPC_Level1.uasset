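; BP_NPC_Level1 is an NPC Blueprint that sends the player to LevelTwo when they enter its interaction zone.
; The InteractionZone overlap accepts only BP_Character and flags the player as nearby.
; It then copies the character's Health and Stamina into BP_GameInstance before opening the level by name, so the values survive the level change.
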(event OnComponentBeginOverlap(InteractionZone)
  (params (OverlappedComponent :type Primitive%20Component%20Object%20Reference) (OtherActor :type Actor%20Object%20Reference) (OtherComp :type Primitive%20Component%20Object%20Reference) (OtherBodyIndex :type Integer) (bFromSweep :type Boolean) (SweepResult :type Hit%20Result%20Structure%20%28by%20ref%29))
  (bind _asbp_character (Utilities|Casting|CastToBP_Character OtherActor))
  (if (== OtherActor _asbp_character)
    (Variables|Default|SetbIsPlayerNearby true)
    (bind _asbp_game_instance (Utilities|Casting|CastToBP_GameInstance (Game|GetGameInstance)))
    (Variables|/Game/Blueprints/BP_GameInstance.BP_GameInstance_C|SetGI_Health _asbp_game_instance (Variables|/Script/FinalProjectPhase2.MyCharacter|GetHealth _asbp_character))
    (Variables|/Game/Blueprints/BP_GameInstance.BP_GameInstance_C|SetGI_Stamina _asbp_game_instance (Variables|/Script/FinalProjectPhase2.MyCharacter|GetStamina _asbp_character))
    (Game|OpenLevel(byName) "LevelTwo")))

(event Collision|EventActorBeginOverlap
  (params (OtherActor :type Actor%20Object%20Reference)))

(event EventTick
  (params (DeltaSeconds :type Float%20%28single-precision%29)))

(fn ConstructionScript)